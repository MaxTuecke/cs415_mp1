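; Spawner actor that builds a chain of tunnel segments, each with a health pack and an enemy.
; On BeginPlay it destroys existing tunnels, then spawns a few, starting at the player and chaining from the newest tunnel's SpawnPoint.
; Each spawn resets the player's HitWall flag, randomizes the wall, and places both pickup and enemy at random offsets.
; Tunnels receive references to the spawner and their spawned actors.
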(event EventBeginPlay
  (CallFunction|SpawnInitalTunnels))

(event Collision|EventActorBeginOverlap
  (params (OtherActor :type Actor%20Object%20Reference)))

(event EventTick
  (params (DeltaSeconds :type Float%20%28single-precision%29)))

(fn ConstructionScript)

(fn SpawnTunnel
  (params (SpawnLocation%20 :type Vector) (A :type Float%20%28double-precision%29))
  (Utilities|FlowControl|Sequence
    (:then_0
      (bind _asbp_player (Utilities|Casting|CastToBP_Player (Game|Player|GetPlayerPawn 0)))
      (Variables|/Game/InfiniteMatrix/Blueprints/BP_Player.BP_Player_C|SethitWall _asbp_player false))
    (:then_1
      (bind _returnvalue (Game|SpawnActorfromClass "/Game/InfiniteMatrix/Blueprints/BP_Tunnel.BP_Tunnel_C" (Math|Transform|MakeTransform (Math|Vector|MakeVector (.x SpawnLocation%20) (.y SpawnLocation%20) (.z SpawnLocation%20)) "0, 0, 0" "1.000000,1.000000,1.000000") "Undefined" "MultiplyWithRoot" 0 0))
      (bind _output_get (Variables|Default|SetNewestTunnel _returnvalue))
      (Variables|/Game/InfiniteMatrix/Blueprints/BP_Tunnel.BP_Tunnel_C|SetTunnelSpawner _output_get self)
      (Default|RandomizeWall _output_get)
      (bind _returnvalue_2 (Game|SpawnActorfromClass "/Game/InfiniteMatrix/Blueprints/BP_HealthPack.BP_HealthPack_C" (Math|Transform|MakeTransform (Math|Vector|MakeVector (+ (.x SpawnLocation%20) (Math|Random|RandomFloatinRange 5e+02 2e+03)) (+ (.y SpawnLocation%20) (Math|Random|RandomFloatinRange -2e+02 2e+02)) (+ (.z SpawnLocation%20) (Math|Random|RandomFloatinRange -2e+02 2e+02))) "0, 0, 0" "1.000000,1.000000,1.000000") "Undefined" "MultiplyWithRoot" 0 0))
      (Variables|/Game/InfiniteMatrix/Blueprints/BP_Tunnel.BP_Tunnel_C|SetHealthPack _output_get _returnvalue_2)
      (bind _returnvalue_3 (Game|SpawnActorfromClass "/Game/InfiniteMatrix/Blueprints/BP_Enemy.BP_Enemy_C" (Math|Transform|MakeTransform (Math|Vector|MakeVector (+ (.x SpawnLocation%20) (Math|Random|RandomFloatinRange 5e+02 2e+03)) (+ (.y SpawnLocation%20) (Math|Random|RandomFloatinRange -2e+02 2e+02)) (+ (.z SpawnLocation%20) (Math|Random|RandomFloatinRange -2e+02 2e+02))) "0, 0, 0" "1.000000,1.000000,1.000000") "Undefined" "MultiplyWithRoot" 0 0))
      (Variables|/Game/InfiniteMatrix/Blueprints/BP_Tunnel.BP_Tunnel_C|SetEnemy _output_get _returnvalue_3))))

(fn SpawnTunnelatSpawnPoint
  (CallFunction|SpawnTunnel (Transformation|GetWorldLocation (Variables|/Game/InfiniteMatrix/Blueprints/BP_Tunnel.BP_Tunnel_C|GetSpawnPoint (Variables|Default|GetNewestTunnel))) 0.0))

(fn SpawnInitalTunnels
  (Utilities|FlowControl|Sequence
    (:then_0
      (bind _outactors (Actor|GetAllActorsOfClass "/Game/InfiniteMatrix/Blueprints/BP_Tunnel.BP_Tunnel_C"))
      (for _array_element _outactors
        (Actor|DestroyActor _array_element)))
    (:then_1
      (for _index (range 0 2)
        (Utilities|IsValid (Variables|Default|GetNewestTunnel)
          (:Is%20Valid
            (CallFunction|SpawnTunnelatSpawnPoint))
          (:Is%20Not%20Valid
            (CallFunction|SpawnTunnel (Transformation|GetActorLocation (Game|Player|GetPlayerPawn 0)) 0.0)))))))