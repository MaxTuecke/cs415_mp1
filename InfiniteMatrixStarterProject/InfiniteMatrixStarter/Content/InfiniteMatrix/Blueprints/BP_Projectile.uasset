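; BP_Projectile is a short-lived projectile that kills enemies and awards score to the player.
; It sets a 1.5-second lifespan on BeginPlay and detects hits through overlaps on its Cone component.
; Overlapping a BP_Enemy adds points to PlayerRef's Score, then destroys both the enemy and the projectile.
; Any other overlap destroys only the projectile, except components named TriggerZone, which it ignores by name comparison.
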(event OnComponentBeginOverlap(Cone)
  (params (OverlappedComponent :type Primitive%20Component%20Object%20Reference) (OtherActor :type Actor%20Object%20Reference) (OtherComp :type Primitive%20Component%20Object%20Reference) (OtherBodyIndex :type Integer) (bFromSweep :type Boolean) (SweepResult :type Hit%20Result%20Structure%20%28by%20ref%29))
  (bind _playerref (Variables|Default|GetPlayerRef))
  (if (Utilities|ClassIsChildOf (Utilities|GetClass OtherActor) "/Game/InfiniteMatrix/Blueprints/BP_Enemy.BP_Enemy_C")
    (Utilities|IsValid self
      (:Is%20Valid
        (Variables|/Game/InfiniteMatrix/Blueprints/BP_Player.BP_Player_C|SetScore _playerref (+ (Variables|/Game/InfiniteMatrix/Blueprints/BP_Player.BP_Player_C|GetScore _playerref) 2.0))
        (Actor|DestroyActor OtherActor)
        (Actor|DestroyActor :!label _label)))
    (elif (not (Utilities|Enum|Equal(Enum) (Utilities|GetObjectName OtherComp) "TriggerZone"))
      (goto _label))))

(event EventBeginPlay
  (Actor|SetLifeSpan 1.5))

(event EventTick
  (params (DeltaSeconds :type Float%20%28single-precision%29)))

(fn ConstructionScript)